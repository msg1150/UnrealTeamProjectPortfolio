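; Plasma gun weapon Blueprint that fires pooled projectiles through multicast spawn events, with damage enabled only where the owner has authority.
; StartFire sets a projectile ID, then either multicasts muzzle aim data or calls the parameterless spawn event, depending on UseMuzzleProjectileAim.
; Both events share one spawn path, selecting between a resolved view start and hit-scan aim.
; Muzzle-aimed shots can converge onto the aim point along the supplied flight direction.
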(event Custom|[M[SpawnProjectile
  (bind _returnvalue (Components|GetOwner))
  (bind (_aimstart _aimend) (CallFunction|GetHitScanAim))
  (bind _weapondata (Variables|Default|GetweaponData))
  (bind _busemuzzleprojectileaim (Variables|Default|GetbUseMuzzleProjectileAim))
  (bind _returnvalue_2 (Class|ProjectilePoolLibrary|SpawnPooledProjectile (Variables|/Game/QuakeLike_1_0/Data/PDA/PDA_WeaponBase.PDA_WeaponBase_C|GetprojectileClass _weapondata) (Math|Transform|MakeTransform (Math|Vector|SelectVector (Class|WeaponProjectileAimLibrary|ResolveProjectileViewStart _returnvalue (CallFunction|SelectMesh) (stale Custom|MulticastMuzzleProjectile ShotStart) (stale Custom|MulticastMuzzleProjectile bCameraFallback)) _aimstart _busemuzzleprojectileaim) (Math|Rotator|FindLookatRotation (Math|Vector|SelectVector (Class|WeaponProjectileAimLibrary|ResolveProjectileViewStart _returnvalue (CallFunction|SelectMesh) (stale Custom|MulticastMuzzleProjectile ShotStart) (stale Custom|MulticastMuzzleProjectile bCameraFallback)) _aimstart _busemuzzleprojectileaim) (Math|Vector|SelectVector (stale Custom|MulticastMuzzleProjectile ShotEnd) _aimend _busemuzzleprojectileaim))) self _weapondata (Game|GetInstigator) (Ability|HasAuthority _returnvalue) (Math|Integer|SelectInt (stale Custom|MulticastMuzzleProjectile ShotId) (Variables|Default|GetprojectileId) _busemuzzleprojectileaim)))
  (Class|WeaponProjectileAimLibrary|ConfigureProjectileConvergence (.AsBP%20Projectile%20Base (Utilities|Casting|CastToBP_ProjectileBase _returnvalue_2)) (stale Custom|MulticastMuzzleProjectile ShotEnd) (stale Custom|MulticastMuzzleProjectile FlightForward) (and (stale Custom|MulticastMuzzleProjectile bConverge) _busemuzzleprojectileaim))
  (Utilities|IsValid (.AsBP%20Projectile%20Base (Utilities|Casting|CastToBP_ProjectileBase _returnvalue_2))))

(event Custom|MulticastMuzzleProjectile
  (params (ShotStart :type Vector) (ShotEnd :type Vector) (ShotId :type Integer) (FlightForward :type Vector) (bConverge :type Boolean) (bCameraFallback :type Boolean))
  (bind _mesh (CallFunction|SelectMesh))
  (bind _returnvalue (Components|GetOwner))
  (bind (_aimstart _aimend) (CallFunction|GetHitScanAim))
  (bind _weapondata (Variables|Default|GetweaponData))
  (bind _busemuzzleprojectileaim (Variables|Default|GetbUseMuzzleProjectileAim))
  (bind _returnvalue_2 (Class|WeaponProjectileAimLibrary|ResolveProjectileViewStart _returnvalue _mesh ShotStart bCameraFallback))
  (bind _returnvalue_3 (Math|Vector|SelectVector _returnvalue_2 _aimstart _busemuzzleprojectileaim))
  (bind _returnvalue_4 (Class|ProjectilePoolLibrary|SpawnPooledProjectile (Variables|/Game/QuakeLike_1_0/Data/PDA/PDA_WeaponBase.PDA_WeaponBase_C|GetprojectileClass _weapondata) (Math|Transform|MakeTransform _returnvalue_3 (Math|Rotator|FindLookatRotation _returnvalue_3 (Math|Vector|SelectVector ShotEnd _aimend _busemuzzleprojectileaim))) self _weapondata (Game|GetInstigator) (Ability|HasAuthority _returnvalue) (Math|Integer|SelectInt ShotId (Variables|Default|GetprojectileId) _busemuzzleprojectileaim)))
  (Class|WeaponProjectileAimLibrary|ConfigureProjectileConvergence (.AsBP%20Projectile%20Base (Utilities|Casting|CastToBP_ProjectileBase _returnvalue_4)) ShotEnd FlightForward (and bConverge _busemuzzleprojectileaim))
  (Utilities|IsValid (.AsBP%20Projectile%20Base (Utilities|Casting|CastToBP_ProjectileBase _returnvalue_4))))

(fn ConstructionScript
  (|CallParentFunction))

(fn StartFire
  (bind (_socketlocation _aimend _flightforward _bconverge _bcamerafallback) (CallFunction|GetProjectileAim))
  (CallFunction|SetProjectileId)
  (if (Variables|Default|GetbUseMuzzleProjectileAim)
    (CallFunction|MulticastMuzzleProjectile _socketlocation _aimend (Variables|Default|GetprojectileId) _flightforward _bconverge _bcamerafallback)
    (else
      (CallFunction|[M[SpawnProjectile))))