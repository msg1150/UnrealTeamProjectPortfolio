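; Rocket launcher projectile that deals direct and radial damage on impact, with knockback that supports rocket jumping.
; On a resolved impact it applies damage through the owning weapon, explodes, requests effects and releases itself.
; The explosion traces from a normal-offset point to target bounds for cover, then scales damage by distance.
; Knockback derives from pre-self-reduction damage, with a self-only Z offset and multiplier, plus a damage-scaled input lock.
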(event OnResolvedImpact(WorldCollision)
  (params (HitComponent :type Primitive%20Component%20Object%20Reference) (OtherActor :type Actor%20Object%20Reference) (OtherComp :type Primitive%20Component%20Object%20Reference) (NormalImpulse :type Vector :default "0, 0, 0") (Hit :type Hit%20Result%20Structure%20%28by%20ref%29))
  (bind (_bblockinghit _binitialoverlap _time _distance _location _impactpoint _normal _impactnormal) (Collision|BreakHitResult Hit))
  (bind _self self)
  (bind _wconfig (Variables|Default|GetwConfig))
  (bind _wconfig_2 (Variables|Default|GetwConfig))
  (Class|ArenaCombatLibrary|RecordTrace self Hit "0, 0, 0" "0, 0, 0")
  (if (Variables|Default|GetcanDealDamage)
    (Utilities|FlowControl|Sequence
      (:then_0
        (Utilities|IsValid (.weapon _wconfig_2)
          (:Is%20Valid
            (Default|[M]DestroyProjectilebyId (.weapon _wconfig_2) (Variables|Default|GetprojectileId) _impactpoint "0, 0, 0"))))
      (:then_1
        (Utilities|FlowControl|Sequence
          (:then_0
            (Utilities|IsValid (.weapon _wconfig)
              (:Is%20Valid
                (Variables|Default|SethitSoundCount 0)
                (Utilities|Array|Clear (Variables|/Game/QuakeLike_1_0/HeldItem/Gun/BP_WeaponBase.BP_WeaponBase_C|GethitInfo (.weapon _wconfig)))
                (Utilities|Casting|CastToCharacter OtherActor)
                (CallFunction|SpawnHitSound 1))))
          (:then_1
            (if (Variables|Default|Getexploded)
              (Class|ProjectilePoolLibrary|ReleaseProjectile)
              (else
                (Variables|Default|Setexploded true)
                (Utilities|IsValid OtherActor
                  (:Is%20Valid
                    (Utilities|IsValid (.weapon _wconfig_2)
                      (:Is%20Valid
                        (Class|ArenaCombatLibrary|BeginProjectileDamage _self)
                        (Default|TakeDamage (.weapon _wconfig_2) (Utilities|Array|MakeArray (Utilities|Struct|MakeST_HitInfo OtherActor (Variables|/Game/QuakeLike_1_0/Data/PDA/PDA_WeaponBase.PDA_WeaponBase_C|Getdamage (.config _wconfig_2)))))
                        (Class|ArenaCombatLibrary|EndProjectileDamage _self))))
                  (:Is%20Not%20Valid
                    _))
                (CallFunction|Explode _impactpoint _impactnormal)
                (Utilities|Casting|CastToCharacter OtherActor
                  (:then
                    (Variables|Default|SetimpactNormalEffect "0, 0, 0"))
                  (:CastFailed
                    (Variables|Default|SetimpactNormalEffect _impactnormal)))
                (Utilities|IsValid (.weapon _wconfig_2)
                  (:Is%20Valid
                    (Default|[M]SpawnDestroyEffect (.weapon _wconfig_2) _impactpoint (Variables|Default|GetimpactNormalEffect) (Class|ProjectileImpactEffectLibrary|GetProjectileImpactWasCharacter (Variables|Default|GetWorldCollision))))
                  (:Is%20Not%20Valid
                    _))
                (Class|ProjectilePoolLibrary|ReleaseProjectile)))))))
    (else
      (Class|ProjectilePoolLibrary|ReleaseProjectile))))

(event OnComponentHit(CollisionComponent)
  (params (HitComponent :type Primitive%20Component%20Object%20Reference) (OtherActor :type Actor%20Object%20Reference) (OtherComp :type Primitive%20Component%20Object%20Reference) (NormalImpulse :type Vector :default "0, 0, 0") (Hit :type Hit%20Result%20Structure%20%28by%20ref%29))
  (Class|ArenaCombatLibrary|RecordTrace self Hit "0, 0, 0" "0, 0, 0"))

(event EventBeginPlay
  (if (not (Class|ProjectilePoolLibrary|IsPooledProjectile self))
    (CallFunction|SetProjectileMesh (Variables|Default|GetSkeletalMesh))
    (Audio|Components|Audio|Play (Variables|Default|GetFlightSound) 0.0)))

(event EventEndPlay
  (params (EndPlayReason :type EEndPlayReason%20Enum :default "Destroyed"))
  (bind _flightsound (Variables|Default|GetFlightSound))
  (|CallParentFunction "Destroyed")
  (Audio|Components|Audio|Stop _flightsound)
  (Components|Activation|Deactivate _flightsound))

(fn ConstructionScript
  (|CallParentFunction))

(fn Explode
  (params (explosionLocation :type Vector) (impactNormal :type Vector))
  (bind _self self)
  (bind _wconfig (Variables|Default|GetwConfig))
  (Utilities|FlowControl|Sequence
    (:then_0
      (bind _outactors (Collision|SphereOverlapActors explosionLocation (Variables|/Game/QuakeLike_1_0/Data/PDA/PDA_WeaponBase.PDA_WeaponBase_C|GetexplosionRadius (.config (Variables|Default|GetwConfig))) (Variables|Default|GetobjectTypes) 0))
      (for _array_element _outactors
        (Utilities|IsValid _array_element
          (:Is%20Valid
            (if (CallFunction|CanExplosionDamageTarget _array_element (CallFunction|SetTraceStart explosionLocation impactNormal 1e+01))
              (if (> (CallFunction|MakeFinalExplosionDamage _array_element explosionLocation) 0.0)
                (Utilities|IsValid (.weapon _wconfig)
                  (:Is%20Valid
                    (Class|ArenaCombatLibrary|BeginProjectileDamage _self)
                    (Default|TakeDamage (.weapon _wconfig) (Utilities|Array|MakeArray (Utilities|Struct|MakeST_HitInfo _array_element (CallFunction|MakeFinalExplosionDamage _array_element explosionLocation))))
                    (Class|ArenaCombatLibrary|EndProjectileDamage _self)
                    (CallFunction|LaunchCharacter _array_element explosionLocation)))))))))
    (:then_1
      (Utilities|IsValid (.weapon (Variables|Default|GetwConfig))
        (:Is%20Valid
          (CallFunction|MakeDebugLineExplosionRadius explosionLocation)
          (CallFunction|SpawnHitSound (Variables|Default|GethitSoundCount)))))))

(fn LaunchCharacter
  (params (targetActor :type Actor%20Object%20Reference) (explosionLocation :type Vector))
  (bind _as캐릭터 (Utilities|Casting|CastToCharacter targetActor))
  (Character|LaunchCharacter _as캐릭터 (CallFunction|MackLaunchVelocity _as캐릭터 explosionLocation) false false)
  (Class|BPIBodyInfo|SetInputStopTimer(Message) _as캐릭터 (CallFunction|GetMoveLockTime)))

(fn MakeDistance
  (params (targetCharacter :type Actor%20Object%20Reference) (explosionLocation :type Vector))
  (bind _returnvalue (Transformation|GetActorLocation targetCharacter))
  (bind _returnvalue_2 (- _returnvalue explosionLocation))
  (return (Math|Vector|VectorLength _returnvalue_2) _returnvalue_2))

(fn MakeAlpha
  (params (distance :type Float%20%28double-precision%29))
  (return (Math|Float|Clamp(Float) (- 1.0 (/ distance (Variables|/Game/QuakeLike_1_0/Data/PDA/PDA_WeaponBase.PDA_WeaponBase_C|GetexplosionRadius (.config (Variables|Default|GetwConfig))))))))

(fn MakeHorizontalDir
  (params (delta :type Vector))
  (bind (_x _y) (Math|Vector|BreakVector delta))
  (return (Math|Vector|Normalize (Math|Vector|MakeVector _x _y 0.0))))

(fn SelectKnockbackMultiplier
  (params (targetCharacter :type Object%20Object%20Reference))
  (bind _wconfig (Variables|Default|GetwConfig))
  (return (Math|Float|SelectFloat (Variables|/Game/QuakeLike_1_0/Data/PDA/PDA_WeaponBase.PDA_WeaponBase_C|GetselfKnockbackMultiplier (.config _wconfig)) (Variables|/Game/QuakeLike_1_0/Data/PDA/PDA_WeaponBase.PDA_WeaponBase_C|GetotherKnockbackMultiplier (.config _wconfig)) (== targetCharacter (Variables|Default|GetInstigator)))))

(fn SelectDamageMultiplier
  (params (hitActor :type Object%20Object%20Reference))
  (return (Math|Float|SelectFloat 1.0 (Variables|/Game/QuakeLike_1_0/Data/PDA/PDA_WeaponBase.PDA_WeaponBase_C|GetselfDamageMultiplier (.config (Variables|Default|GetwConfig))) (== hitActor (Game|GetInstigator)))))

(fn MakeFinalExplosionDamage
  (params (targetCharacter :type Actor%20Object%20Reference) (explosionLocation :type Vector))
  (bind _wconfig (Variables|Default|GetwConfig))
  (Utilities|IsValid (.weapon _wconfig)
    (:Is%20Valid
      (bind _output_get (Variables|Default|SetexplosionDamage (* (CallFunction|MakeAlpha (.distance (CallFunction|MakeDistance targetCharacter explosionLocation))) (Variables|/Game/QuakeLike_1_0/Data/PDA/PDA_WeaponBase.PDA_WeaponBase_C|GetexplosionDamage (.config _wconfig)))))
      (bind _output_get_2 (Variables|Default|SetknockbackDamage _output_get))
      (if (== targetCharacter (Game|GetInstigator))
        (bind _output_get_3 (Variables|Default|SetexplosionDamage (* (Variables|Default|GetexplosionDamage) (Variables|/Game/QuakeLike_1_0/Data/PDA/PDA_WeaponBase.PDA_WeaponBase_C|GetselfDamageMultiplier (.config _wconfig)))))
        (return _output_get_3)
        (else
          (return _output_get_2))))))

(fn MakeFinalKnockback
  (params (targetCharacter :type Object%20Object%20Reference))
  (return (* (CallFunction|SelectKnockbackMultiplier targetCharacter) (* 5.0 (Variables|Default|GetknockbackDamage)))))

(fn MackLaunchVelocity
  (params (targetCharacter :type Actor%20Object%20Reference) (explosionLocation :type Vector))
  (return (* (CallFunction|MakeKnockbackDir targetCharacter explosionLocation) (* (CallFunction|MakeFinalKnockback targetCharacter) (Variables|/Game/QuakeLike_1_0/Data/PDA/PDA_WeaponBase.PDA_WeaponBase_C|GetexplosionPhysicsForce (.config (Variables|Default|GetwConfig)))))))

(fn MakeDebugLineExplosionRadius
  (params (explosionLocation :type Vector))
  (Rendering|Debug|DrawDebugSphere explosionLocation (Variables|/Game/QuakeLike_1_0/Data/PDA/PDA_WeaponBase.PDA_WeaponBase_C|GetexplosionRadius (.config (Variables|Default|GetwConfig))) 36 "(R=0.000000,G=0.000000,B=0.000000,A=1.000000)" 0.5))

(fn SpawnEffectandSound
  (params (impactPoint :type Vector))
  (bind _wconfig (Variables|Default|GetwConfig))
  (bind _projectilesound (Variables|/Game/QuakeLike_1_0/Data/PDA/PDA_WeaponBase.PDA_WeaponBase_C|GetprojectileSound (.config _wconfig)))
  (bind _projectiledestroyeffect (Variables|/Game/QuakeLike_1_0/Data/PDA/PDA_WeaponBase.PDA_WeaponBase_C|GetprojectileDestroyEffect (.config _wconfig)))
  (Utilities|FlowControl|Sequence
    (:then_0
      (Utilities|IsValid _projectiledestroyeffect
        (:Is%20Valid
          (Effects|SpawnEmitteratLocation _projectiledestroyeffect impactPoint))))
    (:then_1
      (Utilities|IsValid _projectilesound
        (:Is%20Valid
          (Audio|SpawnSoundatLocation _projectilesound impactPoint "0, 0, 0" 1.0 1.0 0.0 0 0))))))

(fn CanExplosionDamageTarget
  (params (targetActor :type Actor%20Object%20Reference) (explosionLocation :type Vector))
  (bind _asbp_shooter_base (Utilities|Casting|CastToBP_ShooterBase targetActor))
  (bind _bounds (Class|BPIBodyInfo|GetBounds(Message) _asbp_shooter_base))
  (for _array_element _bounds
    (bind (_outhit _returnvalue) (Collision|LineTraceByChannel explosionLocation _array_element "TraceTypeQuery2" false 0 "None" true "(R=1.000000,G=0.000000,B=0.000000,A=1.000000)" "(R=0.000000,G=1.000000,B=0.000000,A=1.000000)" 0.0))
    (if (and _returnvalue (== targetActor (.HitActor (Collision|BreakHitResult _outhit))))
      (Variables|Default|SethitSoundCount (+ (Variables|Default|GethitSoundCount) 1))
      (return true)))
  (return false))

(fn SetTraceStart
  (params (impactPoint :type Vector) (impactNormal :type Vector) (offset :type Float%20%28double-precision%29))
  (return (+ impactPoint (* offset impactNormal))))

(fn MakeCapsuleSurfaceDistance
  (params (targetCharacter :type Character%20Object%20Reference) (explosionLocation :type Vector))
  (bind _capsulecomponent (Variables|/Script/Engine.Character|GetCapsuleComponent targetCharacter))
  (bind _returnvalue (Transformation|GetWorldLocation _capsulecomponent))
  (bind _returnvalue_2 (Math|Vector|GetUpVector _capsulecomponent))
  (bind _returnvalue_3 (Components|Capsule|GetScaledCapsuleHalfHeight _capsulecomponent))
  (bind _returnvalue_4 (Components|Capsule|GetScaledCapsuleRadius _capsulecomponent))
  (bind _returnvalue_5 (- _returnvalue_3 _returnvalue_4))
  (bind _returnvalue_6 (* _returnvalue_2 _returnvalue_5))
  (return (Math|Float|Max(Float) (- (Math|Vector|Distance(Vector) explosionLocation (Math|Vector|FindClosestPointonSegment explosionLocation (+ _returnvalue _returnvalue_6) (- _returnvalue _returnvalue_6))) _returnvalue_4) 0.0)))

(fn GetMoveLockTime
  (return (* (* (Variables|Default|GetexplosionDamage) (Variables|/Game/QuakeLike_1_0/Data/PDA/PDA_WeaponBase.PDA_WeaponBase_C|GetlockTimeMultiplier (.config (Variables|Default|GetwConfig)))) 0.001)))

(fn MakeKnockbackDir
  (params (targetCharacter :type Actor%20Object%20Reference) (explosionLocation :type Vector))
  (return (Math|Vector|Normalize (- (+ (Math|Vector|MakeVector 0.0 0.0 (Math|Float|SelectFloat (Variables|/Game/QuakeLike_1_0/Data/PDA/PDA_WeaponBase.PDA_WeaponBase_C|GetrocketJumpZOffset (.config (Variables|Default|GetwConfig))) 0.0 (== targetCharacter (Game|GetInstigator)))) (Transformation|GetActorLocation targetCharacter)) explosionLocation))))