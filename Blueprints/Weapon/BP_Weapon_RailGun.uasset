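; Railgun weapon Blueprint that fires a piercing hitscan shot along the aim line.
; StartFire runs a multi line trace, then LoopPierceMax walks hits up to the pierce limit, recording damage, impact effects and the beam end.
; A fatal hit on a shooter applies the pierce damage multiplier to later hits, while a non-fatal one ends the loop.
; Hit sound, beam and impact effects play afterward.
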(event EventStartAbility
  (|CallParentFunction))

(event EventStopAbility
  (|CallParentFunction))

(fn ConstructionScript
  (|CallParentFunction))

(fn StartFire
  (bind (_aimstart _aimend) (CallFunction|GetHitScanAim))
  (Utilities|FlowControl|Sequence
    (:then_0
      (CallFunction|SetHitScan))
    (:then_1
      (Variables|Default|SettraceEnd _aimend)
      (bind _outhits (Collision|MultiLineTraceByChannel _aimstart _aimend (Variables|/Game/QuakeLike_1_0/Data/PDA/PDA_WeaponBase.PDA_WeaponBase_C|GettraceChannel (Variables|Default|GetweaponData)) false (Utilities|Array|MakeArray (Components|GetOwner)) "None"))
      (if (> (Utilities|Array|Length _outhits) 0)
        (Variables|Default|SetbPierce false)
        (CallFunction|LoopPierceMax _outhits (Utilities|Array|Length _outhits))
        (else
          (Variables|Default|SetrailGunBeamEnd (Variables|Default|GettraceEnd)))))
    (:then_2
      (CallFunction|[C]ChHitSound (Variables|Default|GethitSoundCount))
      (CallFunction|[M]HitScanBeamEffect (Variables|Default|GetrailGunBeamEnd) "RailGun")
      (CallFunction|[M]HitEffect (Variables|Default|GeteffectVector)))))

(fn SetFinalDamage
  (bind _weapondata (Variables|Default|GetweaponData))
  (bind _damage (Variables|/Game/QuakeLike_1_0/Data/PDA/PDA_WeaponBase.PDA_WeaponBase_C|Getdamage _weapondata))
  (Variables|Default|SetfinalRailGunDamage (Math|Float|SelectFloat (* (Variables|/Game/QuakeLike_1_0/Data/PDA/PDA_WeaponBase.PDA_WeaponBase_C|GetpierceMultiplier _weapondata) _damage) _damage (Variables|Default|GetbPierce))))

(fn LoopPierceMax
  (params (hits :type Array%20of%20Hit%20Result%20Structures) (length :type Integer))
  (bind _index (Utilities|FlowControl|ForLoopwithBreak 0 (Variables|/Game/QuakeLike_1_0/Data/PDA/PDA_WeaponBase.PDA_WeaponBase_C|GetpierceMax (Variables|Default|GetweaponData)))
    (:LoopBody
      (if (< _index length)
        (Utilities|FlowControl|Sequence
          (:then_0
            (Variables|Default|SetrailGunBeamEnd (.ImpactPoint (Collision|BreakHitResult (Utilities|Array|Get(acopy) hits _index))))
            (Utilities|Array|Add (Variables|Default|GeteffectVector) (Utilities|Struct|MakeST_HitEffectVector (.ImpactPoint (Collision|BreakHitResult (Utilities|Array|Get(acopy) hits _index))) (.ImpactNormal (Collision|BreakHitResult (Utilities|Array|Get(acopy) hits _index)))))
            (CallFunction|SetFinalDamage))
          (:then_1
            (Utilities|IsValid (.HitActor (Collision|BreakHitResult (Utilities|Array|Get(acopy) hits _index)))
              (:Is%20Valid
                (Utilities|Array|Add (Variables|Default|GethitInfo) (Utilities|Struct|MakeST_HitInfo (.HitActor (Collision|BreakHitResult (Utilities|Array|Get(acopy) hits _index))) (Variables|Default|GetfinalRailGunDamage))))))
          (:then_2
            (bind _asbp_shooter_base (Utilities|Casting|CastToBP_ShooterBase (.HitActor (Collision|BreakHitResult (Utilities|Array|Get(acopy) hits _index)))))
            (Variables|Default|SethitSoundCount (+ (Variables|Default|GethitSoundCount) 1))
            (if (Default|IsFatalDamage (Actor|GetComponentbyClass _asbp_shooter_base "/Game/QuakeLike_1_0/Life/BPC_Life.BPC_Life_C") (Variables|Default|GetfinalRailGunDamage))
              (Variables|Default|SetbPierce true)
              (else
                (return)))))
        (else
          (return))))))