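; BP_PistolProjectile is a pistol projectile that reports hits back to its weapon and destroys itself on impact.
; On a collision component hit, only the network authority acts.
; If damage is allowed and the weapon in WConfig is valid, it passes the hit actor and configured damage to that weapon's CallOnHit.
; The projectile is then destroyed whether or not damage was reported.
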(event OnComponentHit(CollisionComponent)
  (params (HitComponent :type Primitive%20Component%20Object%20Reference) (OtherActor :type Actor%20Object%20Reference) (OtherComp :type Primitive%20Component%20Object%20Reference) (NormalImpulse :type Vector :default "0, 0, 0") (Hit :type Hit%20Result%20Structure%20%28by%20ref%29))
  (bind _wconfig (Variables|Default|GetwConfig))
  (Networking|SwitchHasAuthority
    (:Authority
      (if (Variables|Default|GetcanDealDamage)
        (Utilities|IsValid (.weapon _wconfig)
          (:Is%20Valid
            (Default|CallOnHit (.weapon _wconfig) (Utilities|Array|MakeArray (Utilities|Struct|MakeST_HitInfo (.hitactor Hit) (Variables|/Game/QuakeLike_1_0/Data/PDA/PDA_WeaponBase.PDA_WeaponBase_C|Getdamage (.config _wconfig))))))
          (:Is%20Not%20Valid
            _)))
      (Actor|DestroyActor))))

(fn ConstructionScript
  (|CallParentFunction))