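; Shotgun weapon Blueprint that fires a hitscan spread of pellets from the aim point.
; StartFire line-traces each pellet along a random direction in a spread cone around the base aim vector, ignoring the owner.
; Hit actors are recorded in HitInfo with damage that falls off linearly with distance, using WeaponData.
; After all pellets, it passes the Character hit count to CChHitSound and the impact points and normals to MHitEffect.
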(fn ConstructionScript
  (|CallParentFunction))

(fn StartFire
  (bind _aimstart (CallFunction|GetHitScanAim))
  (Utilities|FlowControl|Sequence
    (:then_0
      (CallFunction|SetHitScan)
      (CallFunction|SetBase))
    (:then_1
      (for _index (range 0 (- (Variables|/Game/QuakeLike_1_0/Data/PDA/PDA_WeaponBase.PDA_WeaponBase_C|Getpellet (Variables|Default|GetweaponData)) 1))
        (Utilities|FlowControl|Sequence
          (:then_0
            (CallFunction|SetPelletDirection))
          (:then_1
            (bind (_outhit _returnvalue) (Collision|LineTraceByChannel _aimstart (+ _aimstart (* (Variables|Default|GetpelletDirection) (Variables|Default|GetbaseDistance))) (Variables|/Game/QuakeLike_1_0/Data/PDA/PDA_WeaponBase.PDA_WeaponBase_C|GettraceChannel (Variables|Default|GetweaponData)) false (Utilities|Array|MakeArray (Components|GetOwner)) "None" true "(R=1.000000,G=0.000000,B=0.000000,A=1.000000)" "(R=0.000000,G=1.000000,B=0.000000,A=1.000000)" 0.0))
            (if _returnvalue
              (Utilities|Array|Add (Variables|Default|GeteffectVector) (Utilities|Struct|MakeST_HitEffectVector (.ImpactPoint (Collision|BreakHitResult _outhit)) (.ImpactNormal (Collision|BreakHitResult _outhit))))
              (Utilities|IsValid (.HitActor (Collision|BreakHitResult _outhit))
                (:Is%20Valid
                  (Utilities|Array|Add (Variables|Default|GethitInfo) (Utilities|Struct|MakeST_HitInfo (.HitActor (Collision|BreakHitResult _outhit)) (CallFunction|GetDamage (.Distance (Collision|BreakHitResult _outhit)))))
                  (Utilities|Casting|CastToCharacter (.HitActor (Collision|BreakHitResult _outhit)))
                  (Variables|Default|SethitSoundCount (+ (Variables|Default|GethitSoundCount) 1)))))))))
    (:then_2
      (CallFunction|[C]ChHitSound (Variables|Default|GethitSoundCount))
      (CallFunction|[M]HitEffect (Variables|Default|GeteffectVector)))))

(fn SetBase
  (bind (_aimstart _aimend) (CallFunction|GetHitScanAim))
  (bind _output_get (Variables|Default|SetbaseVector (- _aimend _aimstart)))
  (Variables|Default|SetbaseDistance (Math|Vector|VectorLength _output_get))
  (Variables|Default|SetbaseDirection (Math|Vector|Normalize _output_get)))

(fn SetPelletDirection
  (Variables|Default|SetpelletDirection (Math|Random|RandomUnitVectorinConeinDegrees (Variables|Default|GetbaseDirection) (Variables|/Game/QuakeLike_1_0/Data/PDA/PDA_WeaponBase.PDA_WeaponBase_C|Getspread (Variables|Default|GetweaponData)))))

(fn GetDamage
  (params (distance :type Float%20%28double-precision%29))
  (bind _weapondata (Variables|Default|GetweaponData))
  (bind _damage (Variables|/Game/QuakeLike_1_0/Data/PDA/PDA_WeaponBase.PDA_WeaponBase_C|Getdamage _weapondata))
  (return (Math|Float|Lerp _damage (* _damage (Variables|/Game/QuakeLike_1_0/Data/PDA/PDA_WeaponBase.PDA_WeaponBase_C|GetminDamageMultiplier _weapondata)) (Math|Float|MapRangeClamped distance (Variables|/Game/QuakeLike_1_0/Data/PDA/PDA_WeaponBase.PDA_WeaponBase_C|GetfallOffStart _weapondata) (Variables|/Game/QuakeLike_1_0/Data/PDA/PDA_WeaponBase.PDA_WeaponBase_C|Getrange _weapondata) 0.0 1.0))))