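; Weapon component that fires projectiles and teleport-skill projectiles and plays their impact effects.
; Fire multicasts a spawn, so each machine creates its own projectile from the weapon config, with only authority allowed to damage or teleport.
; Teleport shots notify the owner's teleport skill component and attach a travel effect.
; Helpers play impact particles and sound or destroy projectiles by ID, though the code registering spawned projectiles is disconnected.
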(event Custom|[M]%20SpawnProjectile
  (params (start :type Vector) (end :type Vector) (projectileId :type Integer))
  (bind _wconfig (Variables|Default|GetwConfig))
  (Variables|Default|SetprojectileId projectileId)
  (Game|SpawnActorfromClass (Variables|/Game/QuakeLike_1_0/Data/PDA/PDA_WeaponBase.PDA_WeaponBase_C|GetprojectileClass (.config _wconfig)) (Math|Transform|MakeTransform start (Math|Rotator|FindLookatRotation start end)) "Undefined" "MultiplyWithRoot" (.weapon _wconfig) (Utilities|Struct|MakeST_WeaponConfig (.weapon _wconfig) (.config _wconfig)) (Ability|HasAuthority (.weapon _wconfig)) (Variables|Default|GetprojectileId) (Variables|/Script/Engine.Actor|GetInstigator (.weapon _wconfig))))

(event Custom|[M]SpawnTeleportProjectile
  (params (start :type Vector) (end :type Vector) (teleportData :type PDA%20Teleport%20Skill%20Object%20Reference))
  (bind _returnvalue (Components|GetOwner))
  (bind _returnvalue_2 (Components|GetOwner))
  (bind _traveleffect (Variables|/Game/QuakeLike_1_0/Data/PDA/PDA_TeleportSkill.PDA_TeleportSkill_C|GettravelEffect teleportData))
  (bind _returnvalue_3 (Actor|GetComponentbyClass _returnvalue_2 "/Game/QuakeLike_1_0/Skill/BPC_TeleportSkill.BPC_TeleportSkill_C"))
  (Utilities|IsValid teleportData
    (:Is%20Valid
      (bind _aspawn (Utilities|Casting|CastToPawn _returnvalue))
      (bind _returnvalue_4 (Game|SpawnActorfromClass :Class (Variables|/Game/QuakeLike_1_0/Data/PDA/PDA_TeleportSkill.PDA_TeleportSkill_C|GetprojectileClass teleportData) :SpawnTransform (Math|Transform|MakeTransform start (Math|Rotator|FindLookatRotation start end)) :CollisionHandlingOverride "AlwaysSpawn" :TransformScaleMethod "MultiplyWithRoot" :Owner _returnvalue :canTeleport (Ability|HasAuthority _returnvalue) :skillData teleportData :Instigator _aspawn))
      (Utilities|IsValid _returnvalue_4
        (:Is%20Valid
          (Utilities|IsValid _returnvalue_3
            (:Is%20Valid
              (Default|NotifyTeleportProjectileSpawned _returnvalue_3 _returnvalue_4)
              (Utilities|IsValid _traveleffect
                (:Is%20Valid
                  (Effects|SpawnEmitterAttached _traveleffect (Variables|/Script/Engine.Actor|GetRootComponent _returnvalue_4) "None" "0, 0, 0" "0, 0, 0" "1.000000,1.000000,1.000000" "SnapToTarget" false))))))))))

(event EventInitializeConfig
  (params (wConfig :type ST%20Weapon%20Config%20Structure))
  (Networking|SwitchHasAuthority
    (:Authority
      (Variables|Default|SetwConfig wConfig))))

(event EventFire
  (params (start :type Vector :default "0, 0, 0") (end :type Vector :default "0, 0, 0") (projectileId :type Integer))
  (CallFunction|[M]SpawnProjectile start end projectileId))

(fn DestroyProjectilebyId
  (params (projectileId :type Integer) (impactPoint :type Vector))
  (for _array_element (Variables|Default|GetspawnedProjectiles)
    (Variables|Default|SetspawnedProjectile (Utilities|Struct|MakeST_ProjectileInfo (.projectileid _array_element) (.projectile _array_element)))
    (if (== (.projectileid _array_element) projectileId)
      (Utilities|IsValid (.projectile _array_element)
        (:Is%20Valid
          (Transformation|SetActorLocation (.projectile _array_element) impactPoint false true)
          (Actor|DestroyActor (.projectile _array_element))
          (Utilities|Array|RemoveItem (Variables|Default|GetspawnedProjectiles) (Variables|Default|GetspawnedProjectile)))))))

(fn SpawnDestroyEffect
  (params (impactPoint :type Vector) (impactNormal :type Vector) (hitCharacter :type Boolean))
  (bind _wconfig (Variables|Default|GetwConfig))
  (bind (_particleeffect _niagaraeffect) (Class|ProjectileImpactEffectLibrary|SelectProjectileImpactEffects (.config _wconfig) hitCharacter))
  (bind _projectilesound (Variables|/Game/QuakeLike_1_0/Data/PDA/PDA_WeaponBase.PDA_WeaponBase_C|GetprojectileSound (.config _wconfig)))
  (if (Class|ProjectileImpactEffectLibrary|CanPlayProjectileImpactEffects self (.config _wconfig))
    (Utilities|FlowControl|Sequence
      (:then_0
        (Utilities|IsValid _particleeffect
          (:Is%20Valid
            (Effects|SpawnEmitteratLocation _particleeffect impactPoint (Math|Rotator|MakeRotfromX impactNormal)))
          (:Is%20Not%20Valid
            (Utilities|IsValid _niagaraeffect
              (:Is%20Valid
                (Niagara|SpawnSystematLocation _niagaraeffect impactPoint (Math|Rotator|MakeRotfromX impactNormal)))))))
      (:then_1
        (Utilities|IsValid _projectilesound
          (:Is%20Valid
            (Audio|SpawnSoundatLocation _projectilesound impactPoint "0, 0, 0" (Variables|/Game/QuakeLike_1_0/Data/PDA/PDA_WeaponBase.PDA_WeaponBase_C|GetprojectileDestroyVolumeMultiplier (.config _wconfig)) 1.0 0.0 0 0)))))))