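; Base weapon Blueprint for a multiplayer shooter, driven by WeaponData and supporting hitscan and projectile weapons.
; TryUse gates on refire, equip and usability locally, then server TryFire consumes ammo, multicasts effects, calls empty StartFire hook and applies HitInfo damage.
; Damage includes owner buffs, with kills charging teleport skill (marked temporary).
; Helpers resolve camera aim, muzzle-convergent projectile paths and FP/TP meshes; local HUD handles zoom, recoil and hit markers.
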(event Custom|[M]SpawnDestroyEffect
  (params (impactPoint :type Vector) (impactNormal :type Vector))
  (bind _bpc_projectilefire (Variables|Default|GetBPC_ProjectileFire))
  (Utilities|IsValid _bpc_projectilefire
    (:Is%20Valid
      (Utilities|FlowControl|Sequence
        (:then_0
          (Default|SpawnDestroyEffect _bpc_projectilefire impactPoint impactNormal))))))

(event Custom|PlayMontage
  (bind _fpmesh (Class|BPIBodyInfo|GetMeshes(Message) (.itemowner (Variables|Default|GetitemInfo))))
  (Utilities|IsValid _fpmesh
    (:Is%20Valid
      (Animation|Montage|MontagePlay (Components|SkeletalMesh|GetAnimInstance _fpmesh) (Variables|/Game/QuakeLike_1_0/Data/PDA/PDA_HeldItem.PDA_HeldItem_C|GetuseMontage (Variables|Default|GetweaponData)) 1.0 "MontageLength" 0.0 true))))

(event Custom|[M]FireEffect
  (bind _mesh (CallFunction|SelectMesh))
  (bind _mesh_2 (CallFunction|SelectMesh))
  (bind _mesh_3 (CallFunction|SelectMesh))
  (bind _self self)
  (bind _weapondata (Variables|Default|GetweaponData))
  (bind _aftersmokeeffect (Variables|/Game/QuakeLike_1_0/Data/PDA/PDA_WeaponBase.PDA_WeaponBase_C|GetafterSmokeEffect _weapondata))
  (bind _firesound (Variables|/Game/QuakeLike_1_0/Data/PDA/PDA_WeaponBase.PDA_WeaponBase_C|GetfireSound _weapondata))
  (bind _firefx (Variables|/Game/QuakeLike_1_0/Data/PDA/PDA_WeaponBase.PDA_WeaponBase_C|GetfireFX _weapondata))
  (bind _nsfirefx (Variables|/Game/QuakeLike_1_0/Data/PDA/PDA_WeaponBase.PDA_WeaponBase_C|GetNSFireFX _weapondata))
  (Utilities|FlowControl|Sequence
    (:then_0
      (if (not (Class|ProjectileMuzzleFlashLibrary|ShouldUseProjectileMuzzleFlash self))
        (Utilities|FlowControl|Sequence
          (:then_0
            (Utilities|IsValid _nsfirefx
              (:Is%20Valid
                (Utilities|IsValid _mesh_3
                  (:Is%20Valid
                    (bind _returnvalue (Niagara|SpawnSystemAttached _nsfirefx _mesh_3 "Muzzle" "0, 0, 0" "0, 0, 0" "SnapToTarget" true))
                    (Class|ProjectileFirstPersonRenderingComponent|ApplyFirstPersonMuzzleEffect _self _returnvalue))))))
          (:then_1
            (Utilities|IsValid _firefx
              (:Is%20Valid
                (Utilities|IsValid _mesh_2
                  (:Is%20Valid
                    (bind _returnvalue_2 (Effects|SpawnEmitterAttached _firefx _mesh_2 "Muzzle" "0, 0, 0" "0, 0, 0" "1.000000,1.000000,1.000000" "SnapToTarget"))
                    (Class|ProjectileFirstPersonRenderingComponent|ApplyFirstPersonMuzzleEffect _self _returnvalue_2)))))))))
    (:then_1
      (Utilities|IsValid _aftersmokeeffect
        (:Is%20Valid
          (Utilities|IsValid _mesh
            (:Is%20Valid
              (Effects|SpawnEmitterAttached _aftersmokeeffect _mesh (Variables|/Game/QuakeLike_1_0/Data/PDA/PDA_WeaponBase.PDA_WeaponBase_C|GetsmokeEffectSocketName _weapondata) "0, 0, 0" "0, 0, 0" "1.000000,1.000000,1.000000" "SnapToTarget"))))))
    (:then_2
      (Utilities|IsValid _firesound
        (:Is%20Valid
          (Audio|SpawnSoundatLocation _firesound (Transformation|GetSocketLocation (Variables|Default|GetFP_Mesh) "Muzzle") "0, 0, 0" (Variables|/Game/QuakeLike_1_0/Data/PDA/PDA_WeaponBase.PDA_WeaponBase_C|GetfireVolumeMultiplier _weapondata) 1.0 0.0 "/Game/QuakeLike_1_0/HeldItem/SA/SA_WeaponFire.SA_WeaponFire" 0))))))

(event Custom|[S]%20TryFire
  (bind _hitinfo (Variables|Default|GethitInfo))
  (CallFunction|SetCurrentCount)
  (Utilities|FlowControl|Sequence
    (:then_0
      (CallFunction|[M]FireEffect))
    (:then_1
      (CallFunction|StartFire))
    (:then_2
      (if (> (Utilities|Array|Length _hitinfo) 0)
        (CallFunction|TakeDamage _hitinfo)))))

(event Custom|[M]HitScanBeamEffect
  (params (beamEnd :type Vector) (beamPlayback :type EWeaponBeamPlayback%20Enum :default "MachineGun"))
  (bind _mesh (CallFunction|SelectMesh))
  (bind _weapondata (Variables|Default|GetweaponData))
  (Utilities|IsValid _mesh
    (:Is%20Valid
      (Class|WeaponBeamEffectLibrary|PlayHitScanBeam (Transformation|GetSocketLocation _mesh "Muzzle") beamEnd beamPlayback (Variables|/Game/QuakeLike_1_0/Data/PDA/PDA_WeaponBase.PDA_WeaponBase_C|GethitscanBeamEffect _weapondata) 0 1.2e+04 (Variables|/Game/QuakeLike_1_0/Data/PDA/PDA_WeaponBase.PDA_WeaponBase_C|GetRailGunBeamLifeTime _weapondata) 1e+03 (Variables|/Game/QuakeLike_1_0/Data/PDA/PDA_WeaponBase.PDA_WeaponBase_C|GetrailGunTrailEffect _weapondata) (Variables|/Game/QuakeLike_1_0/Data/PDA/PDA_WeaponBase.PDA_WeaponBase_C|GetrailGunSonicBombEffect _weapondata) (Variables|/Game/QuakeLike_1_0/Data/PDA/PDA_WeaponBase.PDA_WeaponBase_C|GetMachineGunBeamLifeTime _weapondata)))))

(event Custom|TakeDamage
  (params (hitInfo :type Array%20of%20ST%20Hit%20Info%20Structures))
  (bind _returnvalue (Components|GetOwner))
  (bind _returnvalue_2 (Actor|GetComponentbyClass _returnvalue "/Game/QuakeLike_1_0/Buff/BPC_Buff.BPC_Buff_C"))
  (for _array_element hitInfo
    (Utilities|IsValid _returnvalue_2
      (:Is%20Valid
        (Variables|Default|SetfinalDamage (Default|CalcAttackBuff _returnvalue_2 (.damage _array_element))))
      (:Is%20Not%20Valid
        (Variables|Default|SetfinalDamage (.damage _array_element))))
    (Game|Damage|ApplyDamage (.hitactor _array_element) (Variables|Default|GetfinalDamage) (Game|GetInstigatorController _returnvalue) _returnvalue)
    ;[0.15 0.15 0.15 0.5] 임시 구현 추후에 Death관련 이벤트 디스패쳐가 생기면 그쪽으로 이전
    (bind _asbp_shooter_base (Utilities|Casting|CastToBP_ShooterBase (.hitactor _array_element)))
    (if (Default|IsFatalDamage (Actor|GetComponentbyClass _asbp_shooter_base "/Game/QuakeLike_1_0/Life/BPC_Life.BPC_Life_C") (Variables|Default|GetfinalDamage))
      (bind _asbp_shooter_base_2 (Utilities|Casting|CastToBP_ShooterBase (Components|GetOwner)))
      (Utilities|IsValid (Variables|/Game/QuakeLike_1_0/Skill/BPC_TeleportSkill.BPC_TeleportSkill_C|GetskillData (Actor|GetComponentbyClass _asbp_shooter_base_2 "/Game/QuakeLike_1_0/Skill/BPC_TeleportSkill.BPC_TeleportSkill_C"))
        (:Is%20Valid
          (Default|AddSkillGaugebyCooldownReduction (Actor|GetComponentbyClass _asbp_shooter_base_2 "/Game/QuakeLike_1_0/Skill/BPC_TeleportSkill.BPC_TeleportSkill_C") (Variables|/Game/QuakeLike_1_0/Data/PDA/PDA_TeleportSkill.PDA_TeleportSkill_C|GetkillCooldownReduce (Variables|/Game/QuakeLike_1_0/Skill/BPC_TeleportSkill.BPC_TeleportSkill_C|GetskillData (Actor|GetComponentbyClass _asbp_shooter_base_2 "/Game/QuakeLike_1_0/Skill/BPC_TeleportSkill.BPC_TeleportSkill_C")))))))))

(event Custom|[C]ChHitSound
  (params (hitSoundCount :type Integer))
  (bind _weapondata (Variables|Default|GetweaponData))
  (bind _chhitsound (Variables|/Game/QuakeLike_1_0/Data/PDA/PDA_WeaponBase.PDA_WeaponBase_C|GetchHitSound _weapondata))
  (if (> hitSoundCount 0)
    (Utilities|IsValid _weapondata
      (:Is%20Valid
        (Utilities|IsValid _chhitsound
          (:Is%20Valid
            (Audio|PlaySound2D _chhitsound (Variables|/Game/QuakeLike_1_0/Data/PDA/PDA_WeaponBase.PDA_WeaponBase_C|GetchHitVolumeMultiplier _weapondata) 1.0 0.0 "/Game/QuakeLike_1_0/HeldItem/SA/SC_HitSound.SC_HitSound" 0)
            (Variables|Default|SethitSoundCount 0)
            (bind _aspawn (Utilities|Casting|CastToPawn (Components|GetOwner)))
            (bind _asbp_quake_player_controller (Utilities|Casting|CastToBP_QuakePlayerController (Pawn|GetController _aspawn)))
            (Utilities|IsValid (Variables|/Game/QuakeLike_1_0/Controller/BP_QuakePlayerController.BP_QuakePlayerController_C|GetLifeAndWeapon _asbp_quake_player_controller)
              (:Is%20Valid
                (Default|PlayCompetitiveHitMarker (Variables|/Game/QuakeLike_1_0/Controller/BP_QuakePlayerController.BP_QuakePlayerController_C|GetLifeAndWeapon _asbp_quake_player_controller))))))))))

(event Custom|[M]DestroyProjectileById
  (params (projectileId :type Integer) (impactPoint :type Vector) (impactNormal :type Vector))
  (Class|WeaponProjectileAimLibrary|DestroyProjectileVisualsbyId self projectileId))

(event Custom|[M]HitEffect
  (params (effectVector :type Array%20of%20ST%20Hit%20Effect%20Vector%20Structures))
  (bind _weapondata (Variables|Default|GetweaponData))
  (bind _hitscanhiteffect (Variables|/Game/QuakeLike_1_0/Data/PDA/PDA_WeaponBase.PDA_WeaponBase_C|GethitscanHitEffect _weapondata))
  (bind _nshitscanhiteffect (Variables|/Game/QuakeLike_1_0/Data/PDA/PDA_WeaponBase.PDA_WeaponBase_C|GetNSHitscanHitEffect _weapondata))
  (Utilities|IsValid _hitscanhiteffect
    (:Is%20Valid
      (for _array_element effectVector
        (Effects|SpawnEmitteratLocation _hitscanhiteffect (.impactpoint _array_element) (Math|Rotator|MakeRotfromX (.impactnormal _array_element)))))
    (:Is%20Not%20Valid
      (Utilities|IsValid _nshitscanhiteffect
        (:Is%20Valid
          (for _array_element_2 effectVector
            (Niagara|SpawnSystematLocation _nshitscanhiteffect (.impactpoint _array_element_2) (Math|Rotator|MakeRotfromX (.impactnormal _array_element_2)))))))))

(event EventStartAbility
  (bind _returnvalue (Components|GetOwner))
  (Utilities|IsValid _returnvalue
    (:Is%20Valid
      (bind _aspawn (Utilities|Casting|CastToPawn _returnvalue))
      (if (Pawn|IsLocallyControlled _aspawn)
        (bind _asbp_quake_player_controller (Utilities|Casting|CastToBP_QuakePlayerController (Pawn|GetController _aspawn)))
        (Utilities|IsValid (Variables|/Game/QuakeLike_1_0/Controller/BP_QuakePlayerController.BP_QuakePlayerController_C|GetLifeAndWeapon _asbp_quake_player_controller)
          (:Is%20Valid
            (Default|EnterCompetitiveZoom (Variables|/Game/QuakeLike_1_0/Controller/BP_QuakePlayerController.BP_QuakePlayerController_C|GetLifeAndWeapon _asbp_quake_player_controller) (Variables|Default|GetweaponData) (Variables|CrosshairSetting|GetbZoomIn) (Variables|CrosshairSetting|GetbUseScope))))))))

(event EventStopAbility
  (bind _returnvalue (Components|GetOwner))
  (Utilities|IsValid _returnvalue
    (:Is%20Valid
      (bind _aspawn (Utilities|Casting|CastToPawn _returnvalue))
      (if (Pawn|IsLocallyControlled _aspawn)
        (bind _asbp_quake_player_controller (Utilities|Casting|CastToBP_QuakePlayerController (Pawn|GetController _aspawn)))
        (Utilities|IsValid (Variables|/Game/QuakeLike_1_0/Controller/BP_QuakePlayerController.BP_QuakePlayerController_C|GetLifeAndWeapon _asbp_quake_player_controller)
          (:Is%20Valid
            (Default|ExitCompetitiveZoom (Variables|/Game/QuakeLike_1_0/Controller/BP_QuakePlayerController.BP_QuakePlayerController_C|GetLifeAndWeapon _asbp_quake_player_controller))))))))

(event EventTryUse
  (bind _weapondata (Variables|Default|GetweaponData))
  (bind _emptyammosound (Variables|/Game/QuakeLike_1_0/Data/PDA/PDA_WeaponBase.PDA_WeaponBase_C|GetemptyAmmoSound _weapondata))
  ;[0.15 0.15 0.15 0.5] 핑이 튈 시 fire가 이상해질 수 있음
  (if (and (CallFunction|CheckRefireRate) (CallFunction|CheckFinishEquipPlay))
    (Variables|Default|SettimeOfLastShot (Utilities|Time|GetGameTimeinSeconds)) ; 현재 시간 저장(로컬)
    (if (CallFunction|CanUse)
      (Utilities|FlowControl|Sequence
        (:then_0
          (CallFunction|[S]TryFire)
          (CallFunction|PlayMontage))
        (:then_1
          (bind _aspawn (Utilities|Casting|CastToPawn (Components|GetOwner)))
          (bind _asbp_quake_player_controller (Utilities|Casting|CastToBP_QuakePlayerController (Pawn|GetController _aspawn)))
          (Utilities|IsValid (Variables|/Game/QuakeLike_1_0/Controller/BP_QuakePlayerController.BP_QuakePlayerController_C|GetLifeAndWeapon _asbp_quake_player_controller)
            (:Is%20Valid
              (Default|PlayCompetitiveCrosshairRecoil (Variables|/Game/QuakeLike_1_0/Controller/BP_QuakePlayerController.BP_QuakePlayerController_C|GetLifeAndWeapon _asbp_quake_player_controller) (Variables|Default|GetweaponData))))))
      (else
        (Utilities|IsValid _weapondata
          (:Is%20Valid
            (Utilities|IsValid _emptyammosound
              (:Is%20Valid
                (Audio|SpawnSoundatLocation _emptyammosound (Transformation|GetSocketLocation (Variables|Default|GetFP_Mesh) "Muzzle") "0, 0, 0" (Variables|/Game/QuakeLike_1_0/Data/PDA/PDA_WeaponBase.PDA_WeaponBase_C|GetemptyAmmoVolumeMultiplier _weapondata) 1.0 0.0 "/Game/QuakeLike_1_0/HeldItem/SA/SA_HeldItem.SA_HeldItem" 0)))))))))

(event EventBeginPlay
  (bind _weapondata (Variables|Default|GetweaponData))
  (|CallParentFunction)
  (Networking|SwitchHasAuthority
    (:Authority
      (Utilities|IsValid _weapondata
        (:Is%20Valid
          (switch Utilities|FlowControl|Switch|SwitchonE_WeaponType (Variables|/Game/QuakeLike_1_0/Data/PDA/PDA_WeaponBase.PDA_WeaponBase_C|GetweaponType _weapondata)
            (:NewEnumerator1
              (Default|InitializeConfig (Variables|Default|GetBPC_ProjectileFire) (Utilities|Struct|MakeST_WeaponConfig self (Variables|Default|GetweaponData))))))))))

(event EventTick
  (params (DeltaSeconds :type Float%20%28single-precision%29)))

(fn ConstructionScript
  (|CallParentFunction))

(fn GetAimEnd
  (params (aimStartPosition :type Vector) (aimRotation :type Rotator))
  (return (+ aimStartPosition (* (Math|Vector|GetForwardVector aimRotation) (Variables|/Game/QuakeLike_1_0/Data/PDA/PDA_WeaponBase.PDA_WeaponBase_C|Getrange (Variables|Default|GetweaponData))))))

(fn GetProjectileAim
  (bind _mesh (CallFunction|SelectMesh))
  (bind _returnvalue (Components|GetOwner))
  (bind _busemuzzleprojectileaim (Variables|Weapon|Projectile|GetbUseMuzzleProjectileAim))
  (bind _projectileconvergencesettings (Variables|Default|GetProjectileConvergenceSettings))
  (bind _returnvalue_2 (Components|GetOwner _mesh))
  (bind (_aimstartposition _aimrotation) (Class|BPIAim|GetAim(Message) (.itemowner (Variables|Default|GetitemInfo))))
  (if _busemuzzleprojectileaim
    (bind (_projectilestart _aimtarget) (Class|WeaponProjectileAimLibrary|ResolveMuzzleProjectileAim _returnvalue_2 _returnvalue _mesh _aimstartposition (CallFunction|GetAimEnd _aimstartposition _aimrotation) (Variables|/Game/QuakeLike_1_0/Data/PDA/PDA_WeaponBase.PDA_WeaponBase_C|GettraceChannel (Variables|Default|GetweaponData)))))
  (return (Math|Vector|SelectVector (.ReturnValue (Class|WeaponProjectileAimLibrary|ResolveSafeProjectileStart _returnvalue_2 _returnvalue _projectileconvergencesettings _aimstartposition _projectilestart)) (Transformation|GetSocketLocation _mesh "Muzzle") _busemuzzleprojectileaim) (Math|Vector|SelectVector (.FlightTarget (Class|WeaponProjectileAimLibrary|ResolveProjectileConvergence _projectileconvergencesettings _mesh _aimstartposition (CallFunction|GetAimEnd _aimstartposition _aimrotation) (.ReturnValue (Class|WeaponProjectileAimLibrary|ResolveSafeProjectileStart _returnvalue_2 _returnvalue _projectileconvergencesettings _aimstartposition _projectilestart)) _aimtarget (.bCameraFallback (Class|WeaponProjectileAimLibrary|ResolveSafeProjectileStart _returnvalue_2 _returnvalue _projectileconvergencesettings _aimstartposition _projectilestart)))) (CallFunction|GetAimEnd _aimstartposition _aimrotation) _busemuzzleprojectileaim) (.FlightForward (Class|WeaponProjectileAimLibrary|ResolveProjectileConvergence _projectileconvergencesettings _mesh _aimstartposition (CallFunction|GetAimEnd _aimstartposition _aimrotation) (.ReturnValue (Class|WeaponProjectileAimLibrary|ResolveSafeProjectileStart _returnvalue_2 _returnvalue _projectileconvergencesettings _aimstartposition _projectilestart)) _aimtarget (.bCameraFallback (Class|WeaponProjectileAimLibrary|ResolveSafeProjectileStart _returnvalue_2 _returnvalue _projectileconvergencesettings _aimstartposition _projectilestart)))) (and _busemuzzleprojectileaim (.bConverge (Class|WeaponProjectileAimLibrary|ResolveProjectileConvergence _projectileconvergencesettings _mesh _aimstartposition (CallFunction|GetAimEnd _aimstartposition _aimrotation) (.ReturnValue (Class|WeaponProjectileAimLibrary|ResolveSafeProjectileStart _returnvalue_2 _returnvalue _projectileconvergencesettings _aimstartposition _projectilestart)) _aimtarget (.bCameraFallback (Class|WeaponProjectileAimLibrary|ResolveSafeProjectileStart _returnvalue_2 _returnvalue _projectileconvergencesettings _aimstartposition _projectilestart))))) (.bCameraFallback (Class|WeaponProjectileAimLibrary|ResolveSafeProjectileStart _returnvalue_2 _returnvalue _projectileconvergencesettings _aimstartposition _projectilestart))))

(fn CheckRefireRate
  (return (>= (- (Utilities|Time|GetGameTimeinSeconds) (Variables|Default|GettimeOfLastShot)) (Variables|/Game/QuakeLike_1_0/Data/PDA/PDA_WeaponBase.PDA_WeaponBase_C|GetfireRate (Variables|Default|GetweaponData)))))

(fn SetCurrentCount
  (if (not (Class|InitialWeaponLibrary|IsDefaultWeapon))
    (CallFunction|Consum 1)))

(fn GetHitScanAim
  (bind (_aimstartposition _aimrotation) (Class|BPIAim|GetAim(Message) (.itemowner (Variables|Default|GetitemInfo))))
  (return _aimstartposition (CallFunction|GetAimEnd _aimstartposition _aimrotation)))

(fn GetEffectAim
  (params (mesh :type Skeletal%20Mesh%20Component%20Object%20Reference))
  (Utilities|IsValid mesh
    (:Is%20Valid
      (bind (_aimstartposition _aimrotation) (Class|BPIAim|GetAim(Message) (.itemowner (Variables|Default|GetitemInfo))))
      (return (Transformation|GetSocketLocation mesh "Muzzle") (CallFunction|GetAimEnd _aimstartposition _aimrotation)))))

(fn SelectMesh
  (bind _iteminfo (Variables|Default|GetitemInfo))
  (Utilities|IsValid (.itemowner _iteminfo)
    (:Is%20Valid
      (bind _ascharacter (Utilities|Casting|CastToCharacter (.itemowner _iteminfo)))
      (if (Pawn|IsLocallyControlled _ascharacter)
        (return (Variables|Default|GetFP_Mesh))
        (else
          (return (Variables|Default|GetTP_Mesh)))))))

(fn CheckFinishEquipPlay
  (return (< (Variables|Default|GetequipPlayTIme) (Utilities|Time|GetGameTimeinSeconds))))

(fn GetHitScanBeamTransform
  (bind _mesh (CallFunction|SelectMesh))
  (bind _iteminfo (Variables|Default|GetitemInfo))
  (Utilities|IsValid (.itemowner _iteminfo)
    (:Is%20Valid
      (bind _aimrotation (Class|BPIAim|GetAim(Message) (.itemowner _iteminfo)))
      (Utilities|IsValid _mesh
        (:Is%20Valid
          (return (Transformation|GetSocketLocation _mesh "Muzzle") _aimrotation))))))

(fn CheckEmptyPistol
  (return (and (<= (.currentusagecount (Variables|Default|GetcurrentUsageCount)) 0) (GameplayTags|HasTag (Variables|/Game/QuakeLike_1_0/Data/PDA/PDA_HeldItem.PDA_HeldItem_C|Getattributes (Variables|Default|GetweaponData)) "(TagName=\"ID.Pistol\")"))))

(fn SpawnRailGunBeamFX
  (params (Location :type Vector) (Target :type Vector%20%28by%20ref%29))
  (bind _returnvalue (Math|Rotator|FindLookatRotation Location Target))
  (bind _weapondata (Variables|Default|GetweaponData))
  (bind _hitscanbeameffect (Variables|/Game/QuakeLike_1_0/Data/PDA/PDA_WeaponBase.PDA_WeaponBase_C|GethitscanBeamEffect _weapondata))
  (bind _railguntraileffect (Variables|/Game/QuakeLike_1_0/Data/PDA/PDA_WeaponBase.PDA_WeaponBase_C|GetrailGunTrailEffect _weapondata))
  (Utilities|FlowControl|Sequence
    (:then_0
      (Utilities|IsValid _hitscanbeameffect
        (:Is%20Valid
          (bind _returnvalue_2 (Niagara|SpawnSystematLocation _hitscanbeameffect Location _returnvalue "1.000000,1.000000,1.000000" true false "None" false))
          (Utilities|IsValid _returnvalue_2
            (:Is%20Valid
              (Class|NiagaraComponent|SetVariablePosition _returnvalue_2 "User.BeamEnd" (Math|Vector|MakeVector (Math|Vector|Distance(Vector) Location Target) 0.0 0.0))
              (Components|Activation|Activate _returnvalue_2 false))))))
    (:then_1
      (Utilities|IsValid _railguntraileffect
        (:Is%20Valid
          (bind _returnvalue_3 (Niagara|SpawnSystematLocation _railguntraileffect Location _returnvalue "1.000000,1.000000,1.000000" true false "None" false))
          (Utilities|IsValid _returnvalue_3
            (:Is%20Valid
              (Class|NiagaraComponent|SetVariablePosition _returnvalue_3 "User.BeamEnd" (Math|Vector|MakeVector (Math|Vector|Distance(Vector) Location Target) 0.0 0.0))
              (Components|Activation|Activate _returnvalue_3 false))))))))

(fn StartFire)

(fn SetHitScan
  (Utilities|Array|Clear (Variables|Default|GethitInfo))
  (Utilities|Array|Clear (Variables|Default|GeteffectVector))
  (Variables|Default|SethitSoundCount 0))

(fn SetProjectileId
  (Variables|Default|SetprojectileId (+ (Variables|Default|GetprojectileId) 1)))

(fn GetFinalDamage
  (params (bDamage :type Float%20%28double-precision%29))
  (return (Math|Float|SelectFloat (* bDamage 1.0) bDamage false)))

(fn GetZoomData
  (bind _weapondata (Variables|Default|GetweaponData))
  (return (Variables|/Game/QuakeLike_1_0/Data/PDA/PDA_WeaponBase.PDA_WeaponBase_C|GetzoomFov _weapondata) (Variables|/Game/QuakeLike_1_0/Data/PDA/PDA_WeaponBase.PDA_WeaponBase_C|GetinterpSpeed _weapondata)))

(fn GetWeaponData
  (return (Variables|Default|GetweaponData)))