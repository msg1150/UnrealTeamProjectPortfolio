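; Pooled plasma projectile that deals direct and optional radial explosion damage on impact, routed through its owning weapon.
; On resolved impact it damages the hit actor, explodes once, plays effects and hit sounds, then releases itself.
; Explosions check line of sight to target bounds points from a normal-offset origin and scale damage linearly with distance.
; Damage drives knockback and input lockout, with separate self multipliers and a Z offset for rocket jumps.
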(event OnComponentHit(CollisionComponent)
  (params (HitComponent :type Primitive%20Component%20Object%20Reference) (OtherActor :type Actor%20Object%20Reference) (OtherComp :type Primitive%20Component%20Object%20Reference) (NormalImpulse :type Vector :default "0, 0, 0") (Hit :type Hit%20Result%20Structure%20%28by%20ref%29))
  (Class|ArenaCombatLibrary|RecordTrace self Hit "0, 0, 0" "0, 0, 0"))

(event OnResolvedImpact(WorldCollision)
  (params (HitComponent :type Primitive%20Component%20Object%20Reference) (OtherActor :type Actor%20Object%20Reference) (OtherComp :type Primitive%20Component%20Object%20Reference) (NormalImpulse :type Vector :default "0, 0, 0") (Hit :type Hit%20Result%20Structure%20%28by%20ref%29))
  (bind _self self)
  (bind _wconfig (Variables|Default|GetwConfig))
  (bind _wconfig_2 (Variables|Default|GetwConfig))
  (bind _buseexplosiondamage (Variables|Projectile|Explosion|GetbUseExplosionDamage))
  (Class|ArenaCombatLibrary|RecordTrace self Hit "0, 0, 0" "0, 0, 0")
  (if (Variables|Default|GetcanDealDamage)
    (Utilities|FlowControl|Sequence
      (:then_0
        (Utilities|IsValid (.weapon _wconfig)
          (:Is%20Valid
            (Default|[M]DestroyProjectilebyId (.weapon _wconfig) (Variables|Default|GetprojectileId) (.impactpoint Hit) "0, 0, 0"))))
      (:then_1
        (if _buseexplosiondamage
          (if (Variables|Projectile|Explosion|Getexploded)
            (Class|ProjectilePoolLibrary|ReleaseProjectile :!label _label)
            (else
              (Variables|Projectile|Explosion|Setexploded true)
              (Variables|Projectile|Explosion|SethitSoundCount 0)
              (Utilities|FlowControl|Sequence :!label _label_2
                (:then_0
                  (Utilities|IsValid (.weapon _wconfig)
                    (:Is%20Valid
                      (Utilities|Array|Clear (Variables|/Game/QuakeLike_1_0/HeldItem/Gun/BP_WeaponBase.BP_WeaponBase_C|GethitInfo (.weapon _wconfig)))
                      (Utilities|Casting|CastToCharacter (.hitactor Hit))
                      (CallFunction|SpawnHitSound 1))))
                (:then_1
                  (Utilities|IsValid (.weapon _wconfig) ; 무기 존재 체크
                    (:Is%20Valid
                      (Class|ArenaCombatLibrary|BeginProjectileDamage _self)
                      (Default|TakeDamage (.weapon _wconfig) (Utilities|Array|MakeArray (Utilities|Struct|MakeST_HitInfo (.hitactor Hit) (Variables|/Game/QuakeLike_1_0/Data/PDA/PDA_WeaponBase.PDA_WeaponBase_C|Getdamage (.config _wconfig)))))
                      (Class|ArenaCombatLibrary|EndProjectileDamage _self)
                      (if _buseexplosiondamage
                        (CallFunction|Explode (.impactpoint Hit) (.impactnormal Hit))))
                    (:Is%20Not%20Valid
                      _))
                  (Utilities|IsValid (.weapon _wconfig_2)
                    (:Is%20Valid
                      (Default|[M]SpawnDestroyEffect (.weapon _wconfig_2) (.impactpoint Hit) (.impactnormal Hit) (Class|ProjectileImpactEffectLibrary|GetProjectileImpactWasCharacter (Variables|Default|GetWorldCollision)))
                      (goto _label)))))))
          (else
            (goto _label_2)))))
    (else
      (goto _label))))

(event EventBeginPlay
  (if (not (Class|ProjectilePoolLibrary|IsPooledProjectile self))
    (CallFunction|SetProjectileMesh (Variables|Default|GetProjectileMesh))))

(fn ConstructionScript
  (|CallParentFunction))

(fn Explode
  (params (explosionLocation :type Vector :default "0, 0, 0") (impactNormal :type Vector :default "0, 0, 0"))
  (bind _self self)
  (bind _wconfig (Variables|Default|GetwConfig))
  (Utilities|FlowControl|Sequence
    (:then_0
      (bind _outactors (Collision|SphereOverlapActors explosionLocation (Variables|/Game/QuakeLike_1_0/Data/PDA/PDA_WeaponBase.PDA_WeaponBase_C|GetexplosionRadius (.config (Variables|Default|GetwConfig))) (Variables|Projectile|Explosion|GetobjectTypes) 0))
      (for _array_element _outactors
        (Utilities|IsValid _array_element
          (:Is%20Valid
            (if (CallFunction|CanExplosionDamageTarget _array_element (CallFunction|SetTraceStart explosionLocation impactNormal 1e+01))
              (if (> (CallFunction|MakeFinalExplosionDamage _array_element explosionLocation) 0.0)
                (Utilities|IsValid (.weapon _wconfig)
                  (:Is%20Valid
                    (Class|ArenaCombatLibrary|BeginProjectileDamage _self)
                    (Default|TakeDamage (.weapon _wconfig) (Utilities|Array|MakeArray (Utilities|Struct|MakeST_HitInfo _array_element (CallFunction|MakeFinalExplosionDamage _array_element explosionLocation))))
                    (Class|ArenaCombatLibrary|EndProjectileDamage _self)
                    (CallFunction|LaunchCharacter _array_element explosionLocation)))))))))
    (:then_1
      (Utilities|IsValid (.weapon (Variables|Default|GetwConfig))
        (:Is%20Valid
          (CallFunction|MakeDebugLineExplosionRadius explosionLocation)
          (CallFunction|SpawnHitSound (Variables|Projectile|Explosion|GethitSoundCount)))))))

(fn LaunchCharacter
  (params (targetActor :type Actor%20Object%20Reference) (explosionLocation :type Vector :default "0, 0, 0"))
  (bind _ascharacter (Utilities|Casting|CastToCharacter targetActor))
  (Character|LaunchCharacter _ascharacter (CallFunction|MackLaunchVelocity _ascharacter explosionLocation) false false)
  (Class|BPIBodyInfo|SetInputStopTimer(Message) _ascharacter (CallFunction|GetMoveLockTime)))

(fn MakeDistance
  (params (targetCharacter :type Actor%20Object%20Reference) (explosionLocation :type Vector :default "0, 0, 0"))
  (bind _returnvalue (Transformation|GetActorLocation targetCharacter))
  (bind _returnvalue_2 (- _returnvalue explosionLocation))
  (return (Math|Vector|VectorLength _returnvalue_2) _returnvalue_2))

(fn MakeAlpha
  (params (distance :type Float%20%28double-precision%29))
  (bind _wconfig (Variables|Default|GetwConfig))
  (bind _explosionradius (Variables|/Game/QuakeLike_1_0/Data/PDA/PDA_WeaponBase.PDA_WeaponBase_C|GetexplosionRadius (.config _wconfig)))
  (if (> _explosionradius 0.0)
    (return (Math|Float|Clamp(Float) (- 1.0 (/ distance _explosionradius))))
    (else
      (return 0.0))))

(fn MakeHorizontalDir
  (params (delta :type Vector :default "0, 0, 0"))
  (bind (_x _y) (Math|Vector|BreakVector delta))
  (return (Math|Vector|Normalize (Math|Vector|MakeVector _x _y 0.0))))

(fn SelectKnockbackMultiplier
  (params (targetCharacter :type Object%20Object%20Reference))
  (bind _wconfig (Variables|Default|GetwConfig))
  (return (Math|Float|SelectFloat (Variables|/Game/QuakeLike_1_0/Data/PDA/PDA_WeaponBase.PDA_WeaponBase_C|GetselfKnockbackMultiplier (.config _wconfig)) (Variables|/Game/QuakeLike_1_0/Data/PDA/PDA_WeaponBase.PDA_WeaponBase_C|GetotherKnockbackMultiplier (.config _wconfig)) (== targetCharacter (Variables|Default|GetInstigator)))))

(fn SelectDamageMultiplier
  (params (hitActor :type Object%20Object%20Reference))
  (return (Math|Float|SelectFloat 1.0 (Variables|/Game/QuakeLike_1_0/Data/PDA/PDA_WeaponBase.PDA_WeaponBase_C|GetselfDamageMultiplier (.config (Variables|Default|GetwConfig))) (== hitActor (Game|GetInstigator)))))

(fn MakeFinalExplosionDamage
  (params (targetCharacter :type Actor%20Object%20Reference) (explosionLocation :type Vector :default "0, 0, 0"))
  (bind _wconfig (Variables|Default|GetwConfig))
  (Utilities|IsValid (.weapon _wconfig)
    (:Is%20Valid
      (bind _output_get (Variables|Projectile|Explosion|SetexplosionDamage (* (CallFunction|MakeAlpha (.distance (CallFunction|MakeDistance targetCharacter explosionLocation))) (Variables|/Game/QuakeLike_1_0/Data/PDA/PDA_WeaponBase.PDA_WeaponBase_C|GetexplosionDamage (.config _wconfig)))))
      (bind _output_get_2 (Variables|Projectile|Explosion|SetknockbackDamage _output_get))
      (if (== targetCharacter (Game|GetInstigator))
        (bind _output_get_3 (Variables|Projectile|Explosion|SetexplosionDamage (* (Variables|Projectile|Explosion|GetexplosionDamage) (Variables|/Game/QuakeLike_1_0/Data/PDA/PDA_WeaponBase.PDA_WeaponBase_C|GetselfDamageMultiplier (.config _wconfig)))))
        (return _output_get_3)
        (else
          (return _output_get_2))))))

(fn MakeFinalKnockback
  (params (targetCharacter :type Object%20Object%20Reference))
  (return (* (CallFunction|SelectKnockbackMultiplier targetCharacter) (* 5.0 (Variables|Projectile|Explosion|GetknockbackDamage)))))

(fn MackLaunchVelocity
  (params (targetCharacter :type Actor%20Object%20Reference) (explosionLocation :type Vector :default "0, 0, 0"))
  (return (* (CallFunction|MakeKnockbackDir targetCharacter explosionLocation) (* (CallFunction|MakeFinalKnockback targetCharacter) (Variables|/Game/QuakeLike_1_0/Data/PDA/PDA_WeaponBase.PDA_WeaponBase_C|GetexplosionPhysicsForce (.config (Variables|Default|GetwConfig)))))))

(fn MakeDebugLineExplosionRadius
  (params (explosionLocation :type Vector :default "0, 0, 0"))
  (Rendering|Debug|DrawDebugSphere explosionLocation (Variables|/Game/QuakeLike_1_0/Data/PDA/PDA_WeaponBase.PDA_WeaponBase_C|GetexplosionRadius (.config (Variables|Default|GetwConfig))) 36 "(R=0.000000,G=0.000000,B=0.000000,A=1.000000)" 0.5))

(fn SpawnEffectandSound
  (params (impactPoint :type Vector :default "0, 0, 0"))
  (bind _wconfig (Variables|Default|GetwConfig))
  (bind _projectilesound (Variables|/Game/QuakeLike_1_0/Data/PDA/PDA_WeaponBase.PDA_WeaponBase_C|GetprojectileSound (.config _wconfig)))
  (bind _projectiledestroyeffect (Variables|/Game/QuakeLike_1_0/Data/PDA/PDA_WeaponBase.PDA_WeaponBase_C|GetprojectileDestroyEffect (.config _wconfig)))
  (Utilities|FlowControl|Sequence
    (:then_0
      (Utilities|IsValid _projectiledestroyeffect
        (:Is%20Valid
          (Effects|SpawnEmitteratLocation _projectiledestroyeffect impactPoint))))
    (:then_1
      (Utilities|IsValid _projectilesound
        (:Is%20Valid
          (Audio|SpawnSoundatLocation _projectilesound impactPoint "0, 0, 0" 1.0 1.0 0.0 0 0))))))

(fn CanExplosionDamageTarget
  (params (targetActor :type Actor%20Object%20Reference) (explosionLocation :type Vector :default "0, 0, 0"))
  (bind _asbp_shooter_base (Utilities|Casting|CastToBP_ShooterBase targetActor))
  (bind _bounds (Class|BPIBodyInfo|GetBounds(Message) _asbp_shooter_base))
  (for _array_element _bounds
    (bind (_outhit _returnvalue) (Collision|LineTraceByChannel explosionLocation _array_element "TraceTypeQuery2" false 0 "None" true "(R=1.000000,G=0.000000,B=0.000000,A=1.000000)" "(R=0.000000,G=1.000000,B=0.000000,A=1.000000)" 0.0))
    (if (and _returnvalue (== targetActor (.HitActor (Collision|BreakHitResult _outhit))))
      (Variables|Projectile|Explosion|SethitSoundCount (+ (Variables|Projectile|Explosion|GethitSoundCount) 1))
      (return (or true false))))
  (return false))

(fn SetTraceStart
  (params (impactPoint :type Vector :default "0, 0, 0") (impactNormal :type Vector :default "0, 0, 0") (offset :type Float%20%28double-precision%29))
  (return (+ impactPoint (* offset impactNormal))))

(fn MakeCapsuleSurfaceDistance
  (params (targetCharacter :type Character%20Object%20Reference) (explosionLocation :type Vector :default "0, 0, 0"))
  (bind _capsulecomponent (Variables|/Script/Engine.Character|GetCapsuleComponent targetCharacter))
  (bind _returnvalue (Transformation|GetWorldLocation _capsulecomponent))
  (bind _returnvalue_2 (Math|Vector|GetUpVector _capsulecomponent))
  (bind _returnvalue_3 (Components|Capsule|GetScaledCapsuleHalfHeight _capsulecomponent))
  (bind _returnvalue_4 (Components|Capsule|GetScaledCapsuleRadius _capsulecomponent))
  (bind _returnvalue_5 (- _returnvalue_3 _returnvalue_4))
  (bind _returnvalue_6 (* _returnvalue_2 _returnvalue_5))
  (return (Math|Float|Max(Float) (- (Math|Vector|Distance(Vector) explosionLocation (Math|Vector|FindClosestPointonSegment explosionLocation (+ _returnvalue _returnvalue_6) (- _returnvalue _returnvalue_6))) _returnvalue_4) 0.0)))

(fn GetMoveLockTime
  (return (* (* (Variables|Projectile|Explosion|GetexplosionDamage) (Variables|/Game/QuakeLike_1_0/Data/PDA/PDA_WeaponBase.PDA_WeaponBase_C|GetlockTimeMultiplier (.config (Variables|Default|GetwConfig)))) 0.001)))

(fn MakeKnockbackDir
  (params (targetCharacter :type Actor%20Object%20Reference) (explosionLocation :type Vector :default "0, 0, 0"))
  (return (Math|Vector|Normalize (- (+ (Math|Vector|MakeVector 0.0 0.0 (Math|Float|SelectFloat (Variables|/Game/QuakeLike_1_0/Data/PDA/PDA_WeaponBase.PDA_WeaponBase_C|GetrocketJumpZOffset (.config (Variables|Default|GetwConfig))) 0.0 (== targetCharacter (Game|GetInstigator)))) (Transformation|GetActorLocation targetCharacter)) explosionLocation))))