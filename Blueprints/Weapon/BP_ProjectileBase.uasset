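; BP_ProjectileBase is the base weapon projectile, flying straight without gravity at the speed set in its weapon config.
; SetProjectileMesh launches it, sets lifespan from range over speed, and hides the mesh until it has travelled the visual forward offset.
; Ignore disables movement collision between the projectile and its instigator, including a BP_ShooterBase capsule.
; SpawnHitSound forwards a hit sound count to the owning weapon.
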(event Custom|SetProjectileMesh
  (params (projectileMesh :type Scene%20Component%20Object%20Reference))
  (bind _projectilemovement (Variables|Default|GetProjectileMovement))
  (bind _wconfig (Variables|Default|GetwConfig))
  (bind _projectilespeed (Variables|/Game/QuakeLike_1_0/Data/PDA/PDA_WeaponBase.PDA_WeaponBase_C|GetprojectileSpeed (.config _wconfig)))
  (Rendering|SetVisibility projectileMesh false true)
  (Variables|/Script/Engine.ProjectileMovementComponent|SetProjectileGravityScale _projectilemovement 0.0)
  (Game|Components|ProjectileMovement|SetVelocityinLocalSpace _projectilemovement (Math|Vector|MakeVector _projectilespeed 0.0 0.0))
  (CallFunction|Ignore)
  (Actor|SetLifeSpan (/ (Variables|/Game/QuakeLike_1_0/Data/PDA/PDA_WeaponBase.PDA_WeaponBase_C|Getrange (.config _wconfig)) _projectilespeed))
  (Utilities|FlowControl|Delay (/ (Variables|/Game/QuakeLike_1_0/Data/PDA/PDA_WeaponBase.PDA_WeaponBase_C|GetprojectileVisualForwardOffset (.config _wconfig)) _projectilespeed))
  (Rendering|SetVisibility projectileMesh true true))

(fn ConstructionScript)

(fn Ignore
  (bind _returnvalue (Game|GetInstigator))
  (Utilities|IsValid _returnvalue
    (:Is%20Valid
      (Collision|IgnoreActorwhenMoving (Variables|Default|GetCollision%20Component) _returnvalue true)
      (bind _asbp_shooter_base (Utilities|Casting|CastToBP_ShooterBase _returnvalue))
      (Collision|IgnoreActorwhenMoving (Variables|/Script/Engine.Character|GetCapsuleComponent _asbp_shooter_base) self true))))

(fn SpawnHitSound
  (params (hitSoundCount :type Integer))
  (bind _wconfig (Variables|Default|GetwConfig))
  (Utilities|IsValid (.weapon _wconfig)
    (:Is%20Valid
      (Default|[C]ChHitSound (.weapon _wconfig) hitSoundCount))))