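; Pistol weapon Blueprint that fires a single hitscan shot and refills its ammo automatically.
; StartFire line-traces along the aim, records damage and impact data, then triggers hit effects and a hit sound that registers Character hits.
; Each ammo consumption restarts the ReloadPistol timer, so the weapon recovers its starting usage count once the reload time passes without further consumption.
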(event Event[S]Consum
  (params (Consum%20Count :type Integer))
  (|CallParentFunction Consum%20Count)
  (Utilities|Time|ClearTimerbyFunctionName 0 "ReloadPistol")
  (Utilities|Time|SetTimerbyFunctionName 0 "ReloadPistol" (Variables|/Game/QuakeLike_1_0/Data/PDA/PDA_WeaponBase.PDA_WeaponBase_C|GetreloadTime (Variables|Default|GetweaponData))))

(fn ConstructionScript
  (|CallParentFunction))

(fn StartFire
  (bind (_aimstart _aimend) (CallFunction|GetHitScanAim))
  (Utilities|FlowControl|Sequence
    (:then_0
      (CallFunction|SetHitScan))
    (:then_1
      (bind (_outhit _returnvalue) (Collision|LineTraceByChannel _aimstart _aimend (Variables|/Game/QuakeLike_1_0/Data/PDA/PDA_WeaponBase.PDA_WeaponBase_C|GettraceChannel (Variables|Default|GetweaponData)) false (Utilities|Array|MakeArray (Components|GetOwner)) "None" true "(R=1.000000,G=0.000000,B=0.000000,A=1.000000)" "(R=0.000000,G=1.000000,B=0.000000,A=1.000000)" 0.0))
      (if _returnvalue
        (Utilities|Array|Add (Variables|Default|GeteffectVector) (Utilities|Struct|MakeST_HitEffectVector (.ImpactPoint (Collision|BreakHitResult _outhit)) (.ImpactNormal (Collision|BreakHitResult _outhit))))
        (Utilities|IsValid (.HitActor (Collision|BreakHitResult _outhit))
          (:Is%20Valid
            (Utilities|Array|Add (Variables|Default|GethitInfo) (Utilities|Struct|MakeST_HitInfo (.HitActor (Collision|BreakHitResult _outhit)) (Variables|/Game/QuakeLike_1_0/Data/PDA/PDA_WeaponBase.PDA_WeaponBase_C|Getdamage (Variables|Default|GetweaponData))))
            (Utilities|Casting|CastToCharacter (.HitActor (Collision|BreakHitResult _outhit)))
            (Variables|Default|SethitSoundCount 1)))))
    (:then_2
      (CallFunction|[C]ChHitSound (Variables|Default|GethitSoundCount))
      (CallFunction|[M]HitEffect (Variables|Default|GeteffectVector)))))

(fn ReloadPistol
  (CallFunction|[S]Recover (Variables|/Game/QuakeLike_1_0/Data/PDA/PDA_HeldItem.PDA_HeldItem_C|GetstartUsageCount (Variables|Default|GetweaponData))))